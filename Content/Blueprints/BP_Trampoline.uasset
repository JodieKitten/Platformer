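; Trampoline actor for a Paper2D game that launches the player character upward when it overlaps the box.
; The overlap overrides the player's Z velocity, swaps to the raised sprite and widens the orthographic camera to zoom out.
; A DoOnce blocks retriggering until a timed delay restores the sprite, re-arms the trampoline and returns the camera width, regardless of landing.
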(event OnComponentBeginOverlap(Box)
  (params (OverlappedComponent :type Primitive%20Component%20Object%20Reference) (OtherActor :type Actor%20Object%20Reference) (OtherComp :type Primitive%20Component%20Object%20Reference) (OtherBodyIndex :type Integer) (bFromSweep :type Boolean) (SweepResult :type Hit%20Result%20Structure%20%28by%20ref%29))
  ;[1 1 1 0.3] Launch Character & Reset Sprite
  (if (== OtherActor (Variables|Default|GetPlayerCharacterRef))
    (Utilities|FlowControl|DoOnce false
      (:Completed
        (Character|LaunchCharacter (Variables|Default|GetPlayerCharacterRef) (Math|Vector|MakeVector 0.0 0.0 (Variables|Default|GetLaunch%20Velocity%20Z)) false true)
        (CallFunction|ChangeCamera true)
        (Rendering|Components|Sprite|SetSprite (Variables|Default|GetPaperSprite) "/Game/Assets/Tiles/TrampolineUp.TrampolineUp")
        (Utilities|FlowControl|Delay (Variables|Default|GetDuration))
        (Rendering|Components|Sprite|SetSprite (Variables|Default|GetPaperSprite) "/Game/Assets/Tiles/Trampoline.Trampoline")
        (CallFunction|ResetTrampoline)
        (CallFunction|ChangeCamera false)))))

(event Custom|ResetTrampoline
  ;[1 1 1 0.3] Launch Character & Reset Sprite
  (Utilities|FlowControl|DoOnce false) ; enters at Reset
)

(event Custom|ChangeCamera
  (params (Airborne? :type Boolean))
  ;[1 1 1 0.3] Zoom Camera Out
  (if Airborne?
    (Class|CameraComponent|SetOrthoWidth (Variables|/Game/Blueprints/BP_2D_Character.BP_2D_Character_C|GetCamera (Variables|Default|GetPlayerCharacterRef)) 1e+03)
    (else
      (Class|CameraComponent|SetOrthoWidth (Variables|/Game/Blueprints/BP_2D_Character.BP_2D_Character_C|GetCamera (Variables|Default|GetPlayerCharacterRef)) 8e+02))))

(event EventBeginPlay
  (|CallParentFunction) ; This node is disabled and will not be called.\nDrag off pins to build functionality.
)

(event Collision|EventActorBeginOverlap
  (params (OtherActor :type Actor%20Object%20Reference))
  (|CallParentFunction OtherActor) ; This node is disabled and will not be called.\nDrag off pins to build functionality.
)

(event EventTick
  (params (DeltaSeconds :type Float%20%28single-precision%29))
  (|CallParentFunction DeltaSeconds) ; This node is disabled and will not be called.\nDrag off pins to build functionality.
)

(fn ConstructionScript
  (|CallParentFunction))