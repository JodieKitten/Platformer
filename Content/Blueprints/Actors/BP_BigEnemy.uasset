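; BP_BigEnemy is an enemy actor that fires projectiles on a repeating timer and damages actors that touch it.
; After an initial delay on BeginPlay, the Fire event spawns a BP_EnemyProjectile at the Scene component's transform, waits, then calls itself to repeat.
; A Box component applies damage to any actor that begins overlapping it.
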(event OnComponentBeginOverlap(Box)
  (params (OverlappedComponent :type Primitive%20Component%20Object%20Reference) (OtherActor :type Actor%20Object%20Reference) (OtherComp :type Primitive%20Component%20Object%20Reference) (OtherBodyIndex :type Integer) (bFromSweep :type Boolean) (SweepResult :type Hit%20Result%20Structure%20%28by%20ref%29))
  (Game|Damage|ApplyDamage OtherActor 1.0 0 0))

(event Custom|Fire
  (Game|SpawnActorfromClass "/Game/Blueprints/DamageDoers/BP_EnemyProjectile.BP_EnemyProjectile_C" (Transformation|GetWorldTransform (Variables|Default|GetScene)) "Undefined" self 0)
  (Utilities|FlowControl|Delay (Variables|Default|GetDuration))
  (CallFunction|Fire))

(event EventBeginPlay
  (|CallParentFunction)
  (Utilities|FlowControl|Delay (Variables|Default|GetDuration))
  (CallFunction|Fire))

(event Collision|EventActorBeginOverlap
  (params (OtherActor :type Actor%20Object%20Reference))
  (|CallParentFunction OtherActor) ; This node is disabled and will not be called.\nDrag off pins to build functionality.
)

(event EventTick
  (params (DeltaSeconds :type Float%20%28single-precision%29))
  (|CallParentFunction DeltaSeconds) ; This node is disabled and will not be called.\nDrag off pins to build functionality.
)

(fn ConstructionScript
  (|CallParentFunction))