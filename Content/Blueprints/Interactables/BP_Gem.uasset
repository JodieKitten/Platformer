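; BP_Gem is a 2D gem interactable that teleports the player on collection.
; When a BP_2D_Character overlaps its Box, it moves that character to the Waypoint's location and rotation, then calls PauseMovement on the separate PlayerCharacterRef.
; The nodes that would destroy the sprite and Box are disconnected, so this graph leaves the gem in place afterwards.
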(event OnComponentBeginOverlap(Box)
  (params (OverlappedComponent :type Primitive%20Component%20Object%20Reference) (OtherActor :type Actor%20Object%20Reference) (OtherComp :type Primitive%20Component%20Object%20Reference) (OtherBodyIndex :type Integer) (bFromSweep :type Boolean) (SweepResult :type Hit%20Result%20Structure%20%28by%20ref%29))
  (bind _waypoint (Variables|Default|GetWaypoint))
  (bind _returnvalue (Transformation|GetWorldTransform _waypoint))
  ;[1 1 1 0.3] Teleport on collection
  (bind _asbp_2d_character (Utilities|Casting|CastToBP_2D_Character OtherActor))
  (Transformation|Teleport _asbp_2d_character (.location _returnvalue) (.rotation _returnvalue))
  (Default|PauseMovement (Variables|Default|GetPlayerCharacterRef)))

(event EventBeginPlay
  (|CallParentFunction))

(fn ConstructionScript
  (|CallParentFunction))