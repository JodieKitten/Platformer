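; Checkpoint interactable that updates the player character's respawn location when touched.
; When the Box overlap begins with the referenced player character, it stores the Scene component's world location as that character's respawn point.
; It also switches its PaperFlipbook to the Checkpoint flipbook and plays the Flap sound at the actor's location.
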(event OnComponentBeginOverlap(Box)
  (params (OverlappedComponent :type Primitive%20Component%20Object%20Reference) (OtherActor :type Actor%20Object%20Reference) (OtherComp :type Primitive%20Component%20Object%20Reference) (OtherBodyIndex :type Integer) (bFromSweep :type Boolean) (SweepResult :type Hit%20Result%20Structure%20%28by%20ref%29))
  (bind _playercharacterref (Variables|Default|GetPlayerCharacterRef))
  ;[1 1 1 0.3] Set Respawn Point
  (if (== OtherActor _playercharacterref)
    (Variables|/Game/Blueprints/Player/BP_2D_Character.BP_2D_Character_C|SetRespawn%20Location _playercharacterref (Transformation|GetWorldLocation (Variables|Default|GetScene)))
    (Sprite|SetFlipbook (Variables|Default|GetPaperFlipbook) "/Game/Assets/Sprites/LevelFlipbooks/Checkpoint.Checkpoint")
    (Audio|PlaySoundatLocation "/Game/SoundEffects/flap.flap" (Transformation|GetActorLocation) "0, 0, 0" 3.0 1.0 0.0 0 0 0 0)))

(fn ConstructionScript
  (|CallParentFunction))