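; Key-and-lock interactable for a 2D Paper2D game where the player finds a key to free a prisoner and win.
; Key overlap sets HasKey on the player, shows a found widget, hides the Gem sprite and removes the key.
; Lock overlap without the key shows a key-needed widget and the Gem.
; With it, the prisoner jumps, a heart appears, and PauseGame shows the win screen and removes the lock, without actually pausing.
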(event OnComponentBeginOverlap(KeyCollision)
  (params (OverlappedComponent :type Primitive%20Component%20Object%20Reference) (OtherActor :type Actor%20Object%20Reference) (OtherComp :type Primitive%20Component%20Object%20Reference) (OtherBodyIndex :type Integer) (bFromSweep :type Boolean) (SweepResult :type Hit%20Result%20Structure%20%28by%20ref%29))
  ;[1 1 1 0.3] Key Collision
  (if (== OtherActor (Variables|Default|GetPlayerCharacterRef))
    (Variables|/Game/Blueprints/Player/BP_2D_Character.BP_2D_Character_C|SetHasKey (Variables|Default|GetPlayerCharacterRef) true)
    (Audio|SpawnSound2D "/Game/SoundEffects/Coins_10.Coins_10" 1.0 1.0 0.0 0)
    (bind _returnvalue (UserInterface|CreateWidget "/Game/UI/WBP_KeyFound.WBP_KeyFound_C"))
    (UserInterface|Viewport|AddtoViewport _returnvalue 0)
    (if (Rendering|IsVisible (Variables|/Game/Blueprints/Actors/BP_MasterActor.BP_MasterActor_C|GetPaperSprite (Variables|Default|GetGem)))
      (Rendering|SetVisibility (Variables|/Game/Blueprints/Actors/BP_MasterActor.BP_MasterActor_C|GetPaperSprite (Variables|Default|GetGem)) false false))
    (Components|DestroyComponent (Variables|Default|GetPaperSprite))
    (Components|DestroyComponent (Variables|Default|GetKeyCollision))))

(event OnComponentBeginOverlap(LockCollision)
  (params (OverlappedComponent :type Primitive%20Component%20Object%20Reference) (OtherActor :type Actor%20Object%20Reference) (OtherComp :type Primitive%20Component%20Object%20Reference) (OtherBodyIndex :type Integer) (bFromSweep :type Boolean) (SweepResult :type Hit%20Result%20Structure%20%28by%20ref%29))
  ;[1 1 1 0.3] Lock Collision
  (if (== OtherActor (Variables|Default|GetPlayerCharacterRef))
    (if (Variables|/Game/Blueprints/Player/BP_2D_Character.BP_2D_Character_C|GetHasKey (Variables|Default|GetPlayerCharacterRef))
      (Audio|SpawnSound2D "/Game/SoundEffects/unlock.unlock" 2.0 1.0 0.0 0)
      (Audio|SpawnSound2D "/Game/SoundEffects/victory.victory" 1.0 1.0 0.0 0)
      (Sprite|SetFlipbook (Variables|Default|GetPrisoner) "/Game/Assets/Sprites/CharacterFlipbooks/PrisonerJump.PrisonerJump")
      (Rendering|SetVisibility (Variables|Default|GetHeartSprite) true false)
      (Variables|Default|SetGotKey false)
      (CallFunction|PauseGame)
      (else
        (bind _returnvalue (UserInterface|CreateWidget "/Game/UI/WBP_KeyNeeded.WBP_KeyNeeded_C"))
        (UserInterface|Viewport|AddtoViewport _returnvalue 0)
        (Rendering|SetVisibility (Variables|/Game/Blueprints/Actors/BP_MasterActor.BP_MasterActor_C|GetPaperSprite (Variables|Default|GetGem)) true false)))))

(event Custom|Pause%20Game
  ;[1 1 1 0.3] Pause Game
  (bind _returnvalue (UserInterface|CreateWidget "/Game/UI/WBP_WinScreen.WBP_WinScreen_C"))
  (UserInterface|Viewport|AddtoViewport _returnvalue 0)
  (Components|DestroyComponent (Variables|Default|GetLockSprite))
  (Components|DestroyComponent (Variables|Default|GetLockCollision)))

(fn ConstructionScript
  (|CallParentFunction))