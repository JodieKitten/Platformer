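; BP_BigEnemy is an enemy that periodically fires projectiles and damages actors on contact.
; After the parent BeginPlay and an initial delay, a self-calling Fire event spawns a BP_EnemyProjectile at the Scene component's transform, owned by the enemy, with a grunt sound.
; Fire repeats on the same Duration delay with no stop condition in this graph.
; Separately, its Box component applies fixed damage to any actor that begins overlapping it.
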(event OnComponentBeginOverlap(Box)
  (params (OverlappedComponent :type Primitive%20Component%20Object%20Reference) (OtherActor :type Actor%20Object%20Reference) (OtherComp :type Primitive%20Component%20Object%20Reference) (OtherBodyIndex :type Integer) (bFromSweep :type Boolean) (SweepResult :type Hit%20Result%20Structure%20%28by%20ref%29))
  ;[1 1 1 0.3] Damage
  (Game|Damage|ApplyDamage OtherActor 1.0 0 0))

(event Custom|Fire
  ;[1 1 1 0.3] Fire/Spawn Projectile & Sound
  (Game|SpawnActorfromClass "/Game/Blueprints/DamageDoers/BP_EnemyProjectile.BP_EnemyProjectile_C" (Transformation|GetWorldTransform (Variables|Default|GetScene)) "Undefined" self 0)
  (Audio|SpawnSoundatLocation "/Game/SoundEffects/grunt.grunt" (Transformation|GetActorLocation) "0, 0, 0" 2.0 1.0 0.0 "/Game/SoundEffects/ShootAttenuation.ShootAttenuation" 0)
  (Utilities|FlowControl|Delay (Variables|Default|GetDuration))
  (CallFunction|Fire))

(event EventBeginPlay
  ;[1 1 1 0.3] Begin Play/Fire
  (|CallParentFunction)
  (Utilities|FlowControl|Delay (Variables|Default|GetDuration))
  (CallFunction|Fire))

(fn ConstructionScript
  (|CallParentFunction))