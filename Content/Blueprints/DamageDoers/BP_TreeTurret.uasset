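; Tree turret actor that fires bird projectiles on a repeating timer.
; After BeginPlay and an initial delay, the Fire event spawns a BP_BirdProjectile at the Scene component's transform, owned by the turret, and plays a shoot sound at the actor's location.
; Fire then waits the same Duration and calls itself, looping with no targeting or stop condition.
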(event Custom|Fire
  ;[1 1 1 0.3] Fire Projectile
  (Game|SpawnActorfromClass "/Game/Blueprints/DamageDoers/BP_BirdProjectile.BP_BirdProjectile_C" (Transformation|GetWorldTransform (Variables|Default|GetScene)) "Undefined" self 0)
  (Audio|SpawnSoundatLocation "/Game/SoundEffects/shoot.shoot" (Transformation|GetActorLocation) "0, 0, 0" 1.0 1.0 0.0 "/Game/SoundEffects/ShootAttenuation.ShootAttenuation" 0)
  (Utilities|FlowControl|Delay (Variables|Default|GetDuration))
  (CallFunction|Fire))

(event EventBeginPlay
  ;[1 1 1 0.3] Begin Play
  (|CallParentFunction)
  (Utilities|FlowControl|Delay (Variables|Default|GetDuration))
  (CallFunction|Fire))

(fn ConstructionScript
  (|CallParentFunction))