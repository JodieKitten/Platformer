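; BP_DroppingSpikes is a spike trap that drops when the player enters its trigger and damages actors touching the spikes.
; On BeginPlay it calls its parent and stores its starting location.
; The trigger adds a projectile movement component at runtime, plays a falling sound, then after a delay spawns a fresh copy at that location.
; The graph never destroys the dropped original.
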(event OnComponentBeginOverlap(Trigger)
  (params (OverlappedComponent :type Primitive%20Component%20Object%20Reference) (OtherActor :type Actor%20Object%20Reference) (OtherComp :type Primitive%20Component%20Object%20Reference) (OtherBodyIndex :type Integer) (bFromSweep :type Boolean) (SweepResult :type Hit%20Result%20Structure%20%28by%20ref%29))
  ;[1 1 1 0.3] Trigger Event
  (if (== OtherActor (Variables|Default|GetPlayerCharacterRef))
    (AddComponent|AddProjectileMovementComponent (Components|GetOwner (Variables|Default|GetPaperSprite)))
    (Audio|SpawnSoundatLocation "/Game/SoundEffects/falling_spikes.falling_spikes" (Transformation|GetActorLocation) "0, 0, 0" 1.0 1.0 0.0 0 0)
    (Utilities|FlowControl|Delay 4.0)
    (Game|SpawnActorfromClass "BP_DroppingSpikes_C" (Math|Conversions|ToTransform(Vector) (Variables|Default|GetStartingLocation)) "Undefined" 0 0)))

(event OnComponentBeginOverlap(Spikes)
  (params (OverlappedComponent :type Primitive%20Component%20Object%20Reference) (OtherActor :type Actor%20Object%20Reference) (OtherComp :type Primitive%20Component%20Object%20Reference) (OtherBodyIndex :type Integer) (bFromSweep :type Boolean) (SweepResult :type Hit%20Result%20Structure%20%28by%20ref%29))
  ;[1 1 1 0.3] Spike Damage
  (Game|Damage|ApplyDamage OtherActor 1.0 0 0))

(event EventBeginPlay
  ;[1 1 1 0.3] Begin Play - Set Location
  (|CallParentFunction)
  (Variables|Default|SetStartingLocation (Transformation|GetActorLocation)))

(fn ConstructionScript
  (|CallParentFunction))