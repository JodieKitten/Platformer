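; BP_Turret is a damage-dealing turret that repeatedly spawns projectiles on a fixed interval.
; BeginPlay calls the parent, waits for Duration, then triggers the Fire event.
; Fire spawns a BP_Projectile at the Scene component's world transform with itself as owner, then re-calls itself after another Duration delay, looping without any targeting or stop condition.
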(event Custom|Fire
  ;[1 1 1 0.3] Fire
  (Game|SpawnActorfromClass "/Game/Blueprints/DamageDoers/BP_Projectile.BP_Projectile_C" (Transformation|GetWorldTransform (Variables|Default|GetScene)) "Undefined" self 0)
  (Utilities|FlowControl|Delay (Variables|Default|GetDuration))
  (CallFunction|Fire))

(event EventBeginPlay
  ;[1 1 1 0.3] Begin Play
  (|CallParentFunction)
  (Utilities|FlowControl|Delay (Variables|Default|GetDuration))
  (CallFunction|Fire))

(fn ConstructionScript
  (|CallParentFunction))