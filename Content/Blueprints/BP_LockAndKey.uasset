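; BP_LockAndKey is a 2D key-and-lock objective that wins the game when the player brings the key to the lock.
; Overlapping the key sets HasKey on the player, shows a key-found widget and destroys the key's sprite and collision.
; Overlapping the lock without the key shows a key-needed widget.
; With the key, WinAndQuit clears the HUD timer, shows the win screen and removes the lock.
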(event OnComponentBeginOverlap(KeyCollision)
  (params (OverlappedComponent :type Primitive%20Component%20Object%20Reference) (OtherActor :type Actor%20Object%20Reference) (OtherComp :type Primitive%20Component%20Object%20Reference) (OtherBodyIndex :type Integer) (bFromSweep :type Boolean) (SweepResult :type Hit%20Result%20Structure%20%28by%20ref%29))
  ;[1 1 1 0.3] Key Collision
  (if (== OtherActor (Variables|Default|GetPlayerCharacterRef))
    (Variables|/Game/Blueprints/BP_2D_Character.BP_2D_Character_C|SetHasKey (Variables|Default|GetPlayerCharacterRef) true)
    (bind _returnvalue (UserInterface|CreateWidget "/Game/UI/WBP_KeyFound.WBP_KeyFound_C"))
    (UserInterface|Viewport|AddtoViewport _returnvalue 0)
    (Components|DestroyComponent (Variables|Default|GetPaperSprite))
    (Components|DestroyComponent (Variables|Default|GetKeyCollision))))

(event OnComponentBeginOverlap(LockCollision)
  (params (OverlappedComponent :type Primitive%20Component%20Object%20Reference) (OtherActor :type Actor%20Object%20Reference) (OtherComp :type Primitive%20Component%20Object%20Reference) (OtherBodyIndex :type Integer) (bFromSweep :type Boolean) (SweepResult :type Hit%20Result%20Structure%20%28by%20ref%29))
  ;[1 1 1 0.3] Lock Collision
  (if (== OtherActor (Variables|Default|GetPlayerCharacterRef))
    (if (Variables|/Game/Blueprints/BP_2D_Character.BP_2D_Character_C|GetHasKey (Variables|Default|GetPlayerCharacterRef))
      (CallFunction|WinandQuit)
      (else
        (bind _returnvalue (UserInterface|CreateWidget "/Game/UI/WBP_KeyNeeded.WBP_KeyNeeded_C"))
        (UserInterface|Viewport|AddtoViewport _returnvalue 0)))))

(event Custom|WinAndQuit
  (bind _playercharacterref (Variables|Default|GetPlayerCharacterRef))
  ;[1 1 1 0.3] Win And Quit Function
  (Utilities|Casting|CastToBP_2D_Character _playercharacterref)
  (Utilities|Time|ClearandInvalidateTimerbyHandle (Variables|/Game/UI/WBP_HUD.WBP_HUD_C|GetTimerEvent (Variables|/Game/Blueprints/BP_2D_Character.BP_2D_Character_C|GetHUD _playercharacterref)))
  (bind _returnvalue (UserInterface|CreateWidget "/Game/UI/WBP_WinScreen.WBP_WinScreen_C"))
  (UserInterface|Viewport|AddtoViewport _returnvalue 0)
  (Components|DestroyComponent (Variables|Default|GetLockSprite))
  (Components|DestroyComponent (Variables|Default|GetLockCollision)))

(fn ConstructionScript
  (|CallParentFunction))